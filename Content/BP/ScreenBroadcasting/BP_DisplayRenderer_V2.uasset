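; Display actor that captures one of eight screens via a screencap media stream and streams it as compressed frame blocks.
; A widget proxy, sized to the source aspect ratio, applies a foveated compression mask, with gaze currently fixed at centre.
; A fixed-rate update splits its render target into a 2x2 or 4x2 grid by core count.
; Thread-pool workers process the blocks, tagged with display, frame and session IDs, under an execution queue.
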(event Custom|StreamDisplayBuffer
  (|MultithreadedBufferStreaming))

(event EventBeginPlay
  (Utilities|FlowControl|Sequence
    (:then_0
      (Initialization|InitializeProperties))
    (:then_1
      (Initialization|InitializeFixedUpdateTimers))
    (:then_2
      (MultiThreading|InitializeBufferBlockPool))))

(event EventTick
  (params (DeltaSeconds :type Float%20%28single-precision%29))
  (Utilities|FlowControl|Sequence
    (:then_0
      (|EyeGazeTesting))
    (:then_1
      (|InitializeRenderTargetOnceValid))))

(event EventEndPlay
  (params (EndPlayReason :type EEndPlayReason%20Enum :default "Destroyed"))
  (MultiThreading|CancelAllCurrentTasks))

(fn ConstructionScript
  (ScreenCapture|DisplayProxy|UpdateDisplayScale))

(fn InitializeProperties
  (ScreenCapture|InitializeScreenCaptureStream)
  ;[0 0 0] Save resoluton based on raw media
  (bind _output_get (Variables|DisplayProperties|SetSourceResolution (Class|MediaPlayer|GetVideoTrackDimensions (Variables|DisplayProperties|GetMediaPlayer) 1)))
  ;[0 0 0] Deterime validity based off of resolution
  (Variables|Core|SetIsValidDisplay (!= _output_get (Utilities|Struct|MakeIntPoint 0 0)))
  (ScreenCapture|InitializeDisplayAspectRatio false)
  (ScreenCapture|DisplayProxy|InitializeDisplayProxyDrawSize)
  (ScreenCapture|DisplayProxy|UpdateDisplayScale)
  (FoveatedCompression|InitializeFoveatedMaskScaling))

(fn InitializeDisplayAspectRatio
  (params (Debug :type Boolean))
  (bind _sourceresolution (Variables|DisplayProperties|GetSourceResolution))
  (bind _sourceresolution_2 (Variables|DisplayProperties|GetSourceResolution))
  (bind _returnvalue (Math|Conversions|ToFloat(Integer) (.y _sourceresolution_2)))
  (bind _returnvalue_2 (Math|Conversions|ToFloat(Integer) (.x _sourceresolution_2)))
  (bind _returnvalue_3 (Math|Conversions|ToFloat(Integer) (.x _sourceresolution_2)))
  (bind _returnvalue_4 (Math|Conversions|ToFloat(Integer) (.y _sourceresolution_2)))
  (bind _returnvalue_5 (Math|Conversions|ToFloat(Integer) (.y _sourceresolution_2)))
  (bind _returnvalue_6 (Math|Conversions|ToFloat(Integer) (.x _sourceresolution_2)))
  (bind _returnvalue_7 (Math|Conversions|ToFloat(Integer) (.x _sourceresolution)))
  (bind _returnvalue_8 (Math|Conversions|ToFloat(Integer) (.y _sourceresolution)))
  (bind _returnvalue_9 (== _returnvalue_7 _returnvalue_8))
  (bind _returnvalue_10 (/ _returnvalue_6 _returnvalue_5))
  (bind _returnvalue_11 (> _returnvalue_3 _returnvalue_4))
  (bind _returnvalue_12 (/ _returnvalue _returnvalue_2))
  (bind _returnvalue_13 (select _returnvalue_11 _returnvalue_10 _returnvalue_12))
  (bind _returnvalue_14 (select _returnvalue_9 1.0 _returnvalue_13))
  ;[0 0 0] Determine aspect ratio from source resolution
  (Variables|DisplayProperties|SetAspectRatio (select (Math|Float|NearlyEqual(Float) _returnvalue_14 1.0 1e-06) "NewEnumerator0" (select (Math|Float|NearlyEqual(Float) _returnvalue_14 1.777778 1e-06) "NewEnumerator1" (select (Math|Float|NearlyEqual(Float) _returnvalue_14 2.388889 1e-06) "NewEnumerator2" "NewEnumerator1")))))

(fn StartExecutionTimeRecord
  (Variables|PerformanceMonitoring|SetTimeExecutionStarted (Math|DateTime|Now)))

(fn EndExecutionTimeRecord
  (return (Math|Conversions|ToFloat(Integer) (.milliseconds (- (Math|DateTime|Now) (Variables|PerformanceMonitoring|GetTimeExecutionStarted))))))

(fn FixedUpdate30)

(fn FixedUpdate60
  (Class|FoveatedCompressionInterface|UpdateFoveatedCompressionMask(Message) (UserInterface|GetWidget (Variables|Default|GetDisplayProxy)) (Variables|EyeGaze|GetEye%20Gaze%20Hit%20Location) (Variables|EyeGaze|GetInner%20Radius) 2.0)
  (CallFunction|StreamDisplayBuffer))

(fn FixedUpdate2
  (Variables|EyeGaze|SetLerpGateEndLocation (Math|Vector2D|MakeVector2D (Math|Random|RandomFloatinRange 0.0 1.0) (Math|Random|RandomFloatinRange 0.0 1.0)))
  (Variables|EyeGaze|SetFoveatedDebugTargetSize (Math|Random|RandomFloatinRange 4.0 4e+01)))

(fn InitializeFoveatedMaskScaling
  (bind _sourceresolution (Variables|DisplayProperties|GetSourceResolution))
  (bind _sourceresolution_2 (Variables|DisplayProperties|GetSourceResolution))
  (bind _sourceresolution_3 (Variables|DisplayProperties|GetSourceResolution))
  (bind _sourceresolution_4 (Variables|DisplayProperties|GetSourceResolution))
  (Class|FoveatedCompressionInterface|UpdateFoveatedMaskScaling(Message) (UserInterface|GetWidget (Variables|Default|GetDisplayProxy)) (select (== (.x _sourceresolution_3) (.y _sourceresolution_3)) "(X=1.000000,Y=1.000000)" (select (> (.x _sourceresolution_4) (.y _sourceresolution_4)) (Math|Vector2D|MakeVector2D (/ (Math|Conversions|ToFloat(Integer) (.y _sourceresolution)) (Math|Conversions|ToFloat(Integer) (.x _sourceresolution))) 1.0) (Math|Vector2D|MakeVector2D 1.0 (/ (Math|Conversions|ToFloat(Integer) (.x _sourceresolution_2)) (Math|Conversions|ToFloat(Integer) (.y _sourceresolution_2))))))))

(fn UpdateDisplayScale
  (bind _displayproxy (Variables|Default|GetDisplayProxy))
  (bind _sourceresolution (Variables|DisplayProperties|GetSourceResolution))
  (bind _sourceresolution_2 (Variables|DisplayProperties|GetSourceResolution))
  (bind _returnvalue (Class|WidgetComponent|GetDrawSize _displayproxy))
  (bind _returnvalue_2 (/ 1e+02 (.y _returnvalue)))
  (bind _returnvalue_3 (Math|Conversions|ToVector(Float) _returnvalue_2))
  ;[0 0 0] Scale the plane based on the aspect ratio of the display
  (Transformation|SetRelativeScale3D (Variables|Default|GetDisplayRoot) (select (== (.x _sourceresolution_2) (.y _sourceresolution_2)) _returnvalue_3 (select (> (.x _sourceresolution) (.y _sourceresolution)) (Math|Conversions|ToVector(Float) (/ 1e+02 (.x _returnvalue))) _returnvalue_3))))

(fn InitializeDisplayProxyDrawSize
  (Class|WidgetComponent|SetDrawSize (Variables|Default|GetDisplayProxy) (Utilities|Select :Index (Variables|DisplayProperties|GetAspectRatio) :NewEnumerator0 "(X=1080.000000,Y=1080.000000)" :NewEnumerator1 "(X=1920.000000,Y=1080.000000)" :NewEnumerator2 "(X=2560.000000,Y=1080.000000)")))

(fn InitializeScreenCaptureStream
  ;[0 0 0] Set the corresponding media player and media texture material parameter
  (Variables|DisplayProperties|SetMediaPlayer (Utilities|Select :Index (Variables|DisplayProperties|GetDisplay) :NewEnumerator0 "/Game/BP/ScreenBroadcasting/Media/Display/01/MP_Display_01.MP_Display_01" :NewEnumerator1 "/Game/BP/ScreenBroadcasting/Media/Display/02/MP_Display_02.MP_Display_02" :NewEnumerator2 "/Game/BP/ScreenBroadcasting/Media/Display/03/MP_Display_03.MP_Display_03" :NewEnumerator3 "/Game/BP/ScreenBroadcasting/Media/Display/04/MP_Display_04.MP_Display_04" :NewEnumerator4 "/Game/BP/ScreenBroadcasting/Media/Display/05/MP_Display_05.MP_Display_05" :NewEnumerator5 "/Game/BP/ScreenBroadcasting/Media/Display/06/MP_Display_06.MP_Display_06" :NewEnumerator6 "/Game/BP/ScreenBroadcasting/Media/Display/07/MP_Display_07.MP_Display_07" :NewEnumerator7 "/Game/BP/ScreenBroadcasting/Media/Display/08/MP_Display_08.MP_Display_08"))
  (Class|FoveatedCompressionInterface|UpdateMediaSourceTexture(Message) (UserInterface|GetWidget (Variables|Default|GetDisplayProxy)) (Utilities|Select :Index (Variables|DisplayProperties|GetDisplay) :NewEnumerator0 "/Game/BP/ScreenBroadcasting/Media/Display/01/MP_Display_01_Video.MP_Display_01_Video" :NewEnumerator1 "/Game/BP/ScreenBroadcasting/Media/Display/02/MP_Display_02_Video.MP_Display_02_Video" :NewEnumerator2 "/Game/BP/ScreenBroadcasting/Media/Display/03/MP_Display_03_Video.MP_Display_03_Video" :NewEnumerator3 "/Game/BP/ScreenBroadcasting/Media/Display/04/MP_Display_04_Video.MP_Display_04_Video" :NewEnumerator4 "/Game/BP/ScreenBroadcasting/Media/Display/05/MP_Display_05_Video.MP_Display_05_Video" :NewEnumerator5 "/Game/BP/ScreenBroadcasting/Media/Display/06/MP_Display_06_Video.MP_Display_06_Video" :NewEnumerator6 "/Game/BP/ScreenBroadcasting/Media/Display/07/MP_Display_07_Video.MP_Display_07_Video" :NewEnumerator7 "/Game/BP/ScreenBroadcasting/Media/Display/08/MP_Display_08_Video.MP_Display_08_Video"))
  ;[0 0 0] Start the correct display stream
  (Class|MediaPlayer|OpenUrl (Variables|DisplayProperties|GetMediaPlayer) (Utilities|String|Append "screencap://" (Utilities|String|EnumtoString (Variables|DisplayProperties|GetDisplay)) "?fps=60&capture_cursor=true"))
  (Media|MediaPlayer|Play (Variables|DisplayProperties|GetMediaPlayer) :!class /Script/MediaAssets.MediaPlayer))

(fn GetUseableThreadsforMultiThreading
  (bind _returnvalue (Class|MultiThreadTaskLibrary|GetNumberOfCoresIncludingHyperthreads))
  (bind _returnvalue_2 (Math|Conversions|ToFloat(Integer) _returnvalue))
  (bind _returnvalue_3 (/ _returnvalue_2 2.0))
  (bind _returnvalue_4 (Math|Float|Truncate _returnvalue_3))
  (return (select (== (Math|Float|%(Float) _returnvalue_3 2.0) 0.0) _returnvalue_4 (+ _returnvalue_4 1))))

(fn GetRenderTarget
  (return (Class|WidgetComponent|GetRenderTarget (Variables|Default|GetDisplayProxy))))

(fn GetWidgetDrawSize
  (bind _displayproxy (Variables|Default|GetDisplayProxy))
  (bind _returnvalue (Class|WidgetComponent|GetDrawSize _displayproxy))
  (return (Utilities|Struct|MakeIntPoint (Math|Float|Truncate (.x _returnvalue)) (Math|Float|Truncate (.y _returnvalue)))))

(fn CancelAllCurrentTasks
  (bind _bufferblocktasks (Variables|Multithreading|Tasks|GetBufferBlockTasks))
  (Utilities|FlowControl|Sequence
    (:then_0
      (if (> (Utilities|Array|Length _bufferblocktasks) 0)
        (for _array_element _bufferblocktasks
          (Class|MultiTask2UtilitiesLibrary|Cancel _array_element))))))

(fn GetBufferGridLayout
  (return (select (== (MultiThreading|GetThreadsAvailableforBufferCompression) 8) (Utilities|Struct|MakeIntPoint 4 2) (Utilities|Struct|MakeIntPoint 2 2))))

(fn GetThreadsAvailableforBufferCompression
  (return (select (>= (MultiThreading|GetUseableThreadsforMultiThreading) 8) 8 4)))

(fn InitializeFixedUpdateTimers
  (Utilities|Time|SetTimerbyEvent (EventDispatchers|CreateEvent :!event FixedUpdate30) 0.033333 true)
  (Utilities|Time|SetTimerbyEvent (EventDispatchers|CreateEvent :!event FixedUpdate2) 0.5 true)
  (Utilities|Time|SetTimerbyEvent (EventDispatchers|CreateEvent :!event FixedUpdate60) 0.016667 true))

(fn InitializeBufferBlockPool
  (bind _returnvalue (Class|MultiThreadTaskLibrary|CreateThreadPool (MultiThreading|GetThreadsAvailableforBufferCompression) 32768 "TimeCritical" "BufferBlockThreadPool"))
  (Variables|Multithreading|Pools|SetBufferBlockThreadPool _returnvalue))

(fn FixedUpdate100)

(fn GetDisplayRenderTarget
  (bind _capturerrendertarget (Variables|DisplayRendering|GetCapturerRenderTarget)
    (:then
      (return _capturerrendertarget true))
    (:else
      (return 0 false))))

(fn InitializeBufferBlockWorker
  (params (DisplayID :type Byte :default 0) (FrameID :type Byte :default 0) (RenderTarget :type Texture%20Render%20Target%202D%20Object%20Reference%20%28by%20ref%29) (GridLayout :type Int%20Point%20Structure) (BlockCoordinate :type Int%20Point%20Structure) (ClientSessionID :type String) (OptionalServerID :type String))
  (return 0))

(fn InitializeFrameDataChunkConstructorProperties
  (params (BufferChunk :type Array%20of%20Bytes) (ChunkIndex :type Integer) (DisplayID :type E_DisplayToRender%20Enum :default "NewEnumerator0") (FrameID :type Byte :default 0) (ClientSessionID :type String) (OptionalServerID :type String))
  (return 0))