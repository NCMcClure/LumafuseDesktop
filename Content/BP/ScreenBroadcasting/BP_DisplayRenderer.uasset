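; Actor prototype that renders a display for screen broadcasting with eye-tracked foveated compression, currently driven by randomized debug gaze.
; Timers run scene capture and the mask update, which draws concentric color-coded circles at the interpolated gaze point.
; Three display-plane materials are built to use that mask as inner, middle and outer regions.
; Screencap streaming, mask and capturer initialization, and threaded LZF buffer compression exist but are unwired.
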(event Custom|CustomEvent_0
  (CallFunction|UpdateFoveatedCompressionMask (Variables|Default|GetEye%20Gaze%20Hit%20Location) (Variables|Default|GetInner%20Radius) 2.0)
  (Rendering|SceneCapture|CaptureScene (Variables|Default|GetCapture) :!class /Script/Engine.SceneCaptureComponent2D))

(event Custom|UpdateDebugEyeLocation
  (Variables|Default|SetLerpGateEndLocation (Math|Vector2D|MakeVector2D (Math|Random|RandomFloatinRange 0.0 1.0) (Math|Random|RandomFloatinRange 0.0 1.0)))
  (Variables|Default|SetFoveatedDebugTargetSize (Math|Random|RandomFloatinRange 4.0 4e+01)))

(event Custom|CustomEvent_1)

(event EventBeginPlay
  (Utilities|FlowControl|Sequence
    (:then_0
      (CallFunction|InitializeProperties)
      (Rendering|SceneCapture|ShowOnlyActorComponents (Variables|Default|GetCapture) self false)
      (Utilities|Array|Resize (Variables|Default|GetBuffer) (* 1920 1080 4))
      (Utilities|Time|SetTimerbyEvent (delegate Custom|CustomEvent_0) 0.033333 true)
      (Utilities|Time|SetTimerbyEvent (delegate Custom|UpdateDebugEyeLocation) 0.5 true)
      (Utilities|Time|SetTimerbyEvent (delegate Custom|CustomEvent_1) 0.016667 true))
    (:then_1
      (Utilities|FlowControl|Delay 1.0)
      (PerformanceMonitoring|StartExecutionTimeRecord))))

(event EventTick
  (params (DeltaSeconds :type Float%20%28single-precision%29))
  (Utilities|FlowControl|Sequence
    (:then_0
      (Variables|Default|SetEye%20Gaze%20Hit%20Location (Math|Conversions|ToVector2D(Vector) (Math|Interpolation|VInterpTo (Math|Conversions|ToVector(Vector2D) (Variables|Default|GetEye%20Gaze%20Hit%20Location)) (Math|Conversions|ToVector(Vector2D) (Variables|Default|GetLerpGateEndLocation)) (Utilities|Time|GetWorldDeltaSeconds) 3.0)))
      (Variables|Default|SetInner%20Radius (Math|Interpolation|FInterpTo (Variables|Default|GetInner%20Radius) (Variables|Default|GetFoveatedDebugTargetSize) (Utilities|Time|GetWorldDeltaSeconds) 1.0)))))

(fn ConstructionScript
  (bind _displayplane_inner (Variables|Default|GetDisplayPlane_Inner))
  (bind _displayplane_middle (Variables|Default|GetDisplayPlane_Middle))
  (bind _displayplane_outer (Variables|Default|GetDisplayPlane_Outer))
  (bind _returnvalue (Rendering|Material|CreateDynamicMaterialInstance _displayplane_inner 0 (Rendering|Material|GetMaterial _displayplane_inner 0) "None" :!class /Script/Engine.PrimitiveComponent))
  (Variables|DisplayProperties|SetDMI_DisplayPlane_Inner _returnvalue)
  (bind _returnvalue_2 (Rendering|Material|CreateDynamicMaterialInstance _displayplane_middle 0 (Rendering|Material|GetMaterial _displayplane_middle 0) "None" :!class /Script/Engine.PrimitiveComponent))
  (Variables|DisplayProperties|SetDMI_DisplayPlane_Middle _returnvalue_2)
  (bind _returnvalue_3 (Rendering|Material|CreateDynamicMaterialInstance _displayplane_outer 0 (Rendering|Material|GetMaterial _displayplane_outer 0) "None" :!class /Script/Engine.PrimitiveComponent))
  (Variables|DisplayProperties|SetDMI_DisplayPlane_Outer _returnvalue_3))

(fn GetResolutionScale
  (return (Variables|DisplayProperties|GetCurrentResolutionScale)))

(fn InitializeProperties
  ;[0 0 0] Set the corresponding media player and media texture material parameter
  (Variables|DisplayProperties|SetMediaPlayer (Utilities|Select :Index (Variables|DisplayProperties|GetDisplay) :NewEnumerator0 "/Game/BP/ScreenBroadcasting/Media/Display/01/MP_Display_01.MP_Display_01" :NewEnumerator1 "/Game/BP/ScreenBroadcasting/Media/Display/02/MP_Display_02.MP_Display_02" :NewEnumerator2 "/Game/BP/ScreenBroadcasting/Media/Display/03/MP_Display_03.MP_Display_03" :NewEnumerator3 "/Game/BP/ScreenBroadcasting/Media/Display/04/MP_Display_04.MP_Display_04" :NewEnumerator4 "/Game/BP/ScreenBroadcasting/Media/Display/05/MP_Display_05.MP_Display_05" :NewEnumerator5 "/Game/BP/ScreenBroadcasting/Media/Display/06/MP_Display_06.MP_Display_06" :NewEnumerator6 "/Game/BP/ScreenBroadcasting/Media/Display/07/MP_Display_07.MP_Display_07" :NewEnumerator7 "/Game/BP/ScreenBroadcasting/Media/Display/08/MP_Display_08.MP_Display_08")))

(fn UpdateResolutionScale
  (params (Scale :type Float%20%28single-precision%29))
  (bind _capture (Variables|Default|GetCapture))
  (bind _sourceresolution (Variables|DisplayProperties|GetSourceResolution))
  (bind _output_get (LocalVariables|SetTempScale (Math|Float|Clamp(Float) Scale)))
  (Variables|DisplayProperties|SetCurrentResolutionScale _output_get)
  (Class|KismetRenderingLibrary|ReleaseRenderTarget2D (Variables|DisplayRendering|GetCapturerRenderTarget))
  (bind _returnvalue (Rendering|CreateRenderTarget2D (Math|Integer|Clamp(Integer) (Math|Float|Truncate (* (LocalVariables|GetTempScale) (Math|Conversions|ToFloat(Integer) (.x _sourceresolution)))) 2 3840) (Math|Integer|Clamp(Integer) (Math|Float|Truncate (* (LocalVariables|GetTempScale) (Math|Conversions|ToFloat(Integer) (.y _sourceresolution)))) 2 3840) "RTF_RGBA8_SRGB"))
  (bind _output_get_2 (Variables|DisplayRendering|SetCapturerRenderTarget _returnvalue))
  (Variables|/Script/Engine.SceneCaptureComponent2D|SetTextureTarget _capture _output_get_2)
  (Rendering|SceneCapture|CaptureScene _capture :!class /Script/Engine.SceneCaptureComponent2D))

(fn InitializeDisplayCapturer
  (params (Debug :type Boolean))
  (bind _sourceresolution (Variables|DisplayProperties|GetSourceResolution))
  (bind _capture (Variables|Default|GetCapture))
  (bind _sourceresolution_2 (Variables|DisplayProperties|GetSourceResolution))
  (bind _returnvalue (Math|Conversions|ToFloat(Integer) (.y _sourceresolution_2)))
  (bind _returnvalue_2 (Math|Conversions|ToFloat(Integer) (.x _sourceresolution_2)))
  (bind _returnvalue_3 (Math|Conversions|ToFloat(Integer) (.x _sourceresolution_2)))
  (bind _returnvalue_4 (Math|Conversions|ToFloat(Integer) (.y _sourceresolution_2)))
  (bind _returnvalue_5 (Math|Conversions|ToFloat(Integer) (.y _sourceresolution_2)))
  (bind _returnvalue_6 (Math|Conversions|ToFloat(Integer) (.x _sourceresolution_2)))
  (bind _returnvalue_7 (Math|Conversions|ToFloat(Integer) (.x _sourceresolution)))
  (bind _returnvalue_8 (Math|Conversions|ToFloat(Integer) (.y _sourceresolution)))
  (bind _returnvalue_9 (== _returnvalue_7 _returnvalue_8))
  (bind _returnvalue_10 (/ _returnvalue_6 _returnvalue_5))
  (bind _returnvalue_11 (> _returnvalue_3 _returnvalue_4))
  (bind _returnvalue_12 (/ _returnvalue _returnvalue_2))
  (bind _returnvalue_13 (select _returnvalue_11 _returnvalue_10 _returnvalue_12))
  (bind _returnvalue_14 (select _returnvalue_9 1.0 _returnvalue_13))
  ;[0 0 0] Determine aspect ratio from source resolution
  (bind _output_get (Variables|DisplayProperties|SetAspectRatio (select (Math|Float|NearlyEqual(Float) _returnvalue_14 1.0 1e-06) "NewEnumerator0" (select (Math|Float|NearlyEqual(Float) _returnvalue_14 1.777778 1e-06) "NewEnumerator1" (select (Math|Float|NearlyEqual(Float) _returnvalue_14 2.388889 1e-06) "NewEnumerator2" "NewEnumerator1")))))
  (bind _output_get_2 (Variables|DisplayProperties|SetRenderResolution (Utilities|Select :Index _output_get :NewEnumerator0 (Utilities|Struct|MakeIntPoint 1080 1080) :NewEnumerator1 (Utilities|Struct|MakeIntPoint 1920 1080) :NewEnumerator2 (Utilities|Struct|MakeIntPoint 2560 1080))))
  (bind _returnvalue_15 (Rendering|CreateRenderTarget2D (.X (Utilities|Struct|BreakIntPoint _output_get_2)) (.Y (Utilities|Struct|BreakIntPoint _output_get_2)) "RTF_RGBA8_SRGB"))
  (bind _output_get_3 (Variables|DisplayRendering|SetCapturerRenderTarget _returnvalue_15))
  (Variables|/Script/Engine.SceneCaptureComponent2D|SetTextureTarget _capture _output_get_3)
  (Rendering|SceneCapture|CaptureScene _capture :!class /Script/Engine.SceneCaptureComponent2D)
  (Rendering|SceneCapture|ShowOnlyActorComponents (Variables|Default|GetCapture) self false))

(fn UpdateFoveatedCompressionMask
  (params (EyeGazeHitLocation :type Vector%202D%20Structure) (InnerRadius :type Float%20%28single-precision%29) (BlendRadiusRatio :type Float%20%28single-precision%29))
  (bind _returnvalue (* InnerRadius BlendRadiusRatio))
  (Variables|Optimization|FoveatedCompression|GetFoveatedCompressionMaskRenderTarget
    (:then
      (Rendering|ClearRenderTarget2D "/Game/BP/ScreenBroadcasting/FoveatedCompression/RT_FoveatedMask.RT_FoveatedMask" "(R=0.000000,G=0.000000,B=1.000000,A=1.000000)")
      (bind (_canvas _size _context) (Rendering|BeginDrawCanvastoRenderTarget "/Game/BP/ScreenBroadcasting/FoveatedCompression/RT_FoveatedMask.RT_FoveatedMask"))
      (LocalVariables|SetCanvasRenderTargetSize _size)
      (LocalVariables|SetCanvasContext _context)
      ;[0 0 0] Draw the middle circle to the canvas first.
      (Canvas|DrawMaterial _canvas (Variables|Optimization|FoveatedCompression|GetDMI_FoveationMask_Middle) (- (* (LocalVariables|GetCanvasRenderTargetSize) EyeGazeHitLocation) (* _returnvalue 0.5)) (Math|Vector2D|MakeVector2D _returnvalue _returnvalue) "(X=0.000000,Y=0.000000)" "(X=1.000000,Y=1.000000)" 0.0 "(X=0.000000,Y=0.000000)")
      ;[0 0 0] Draw the inner radius to the canvas second so that it overlaps the middle
      (Canvas|DrawMaterial _canvas (Variables|Optimization|FoveatedCompression|GetDMI_FoveationMask_Inner) (- (* (LocalVariables|GetCanvasRenderTargetSize) EyeGazeHitLocation) (* InnerRadius 0.5)) (Math|Vector2D|MakeVector2D InnerRadius InnerRadius) "(X=0.000000,Y=0.000000)" "(X=1.000000,Y=1.000000)" 0.0 "(X=0.000000,Y=0.000000)")
      (Rendering|EndDrawCanvastoRenderTarget (LocalVariables|GetCanvasContext)))
    (:else
      (Development|PrintString "FoveatedCompressionRenderTarget is not valid!" true true "(R=1.000000,G=0.000000,B=0.000000,A=1.000000)"))))

(fn StartExecutionTimeRecord
  (Variables|PerformanceMonitoring|SetTimeExecutionStarted (Math|DateTime|Now)))

(fn EndExecutionTimeRecord
  (Development|PrintString (Utilities|String|Append (Utilities|String|ToString(Integer) (.milliseconds (- (Math|DateTime|Now) (Variables|PerformanceMonitoring|GetTimeExecutionStarted)))) "ms") true true "(R=0.000000,G=0.660000,B=1.000000,A=1.000000)" 1e+01))

(fn InitializeFoveationMaskMaterials
  (bind _returnvalue (Rendering|Material|CreateDynamicMaterialInstance "/Game/BP/ScreenBroadcasting/FoveatedCompression/Materials/Masking/M_MaskCircle.M_MaskCircle" "None" "None" :!class /Script/Engine.KismetMaterialLibrary))
  (Rendering|Material|SetVectorParameterValue _returnvalue "Color" "(R=1.000000,G=0.000000,B=0.000000,A=1.000000)" :!class /Script/Engine.MaterialInstanceDynamic)
  (Variables|Optimization|FoveatedCompression|SetDMI_FoveationMask_Inner _returnvalue)
  (bind _returnvalue_2 (Rendering|Material|CreateDynamicMaterialInstance "/Game/BP/ScreenBroadcasting/FoveatedCompression/Materials/Masking/M_MaskCircle.M_MaskCircle" "None" "None" :!class /Script/Engine.KismetMaterialLibrary))
  (Rendering|Material|SetVectorParameterValue _returnvalue_2 "Color" "(R=0.000000,G=1.000000,B=0.000000,A=1.000000)" :!class /Script/Engine.MaterialInstanceDynamic)
  (Variables|Optimization|FoveatedCompression|SetDMI_FoveationMask_Middle _returnvalue_2))

(fn InitializeFoveatedCompressionMaskRenderTarget
  (bind _output_get (Variables|Optimization|FoveatedCompression|SetFoveatedCompressionMaskResolution (Utilities|Select :Index (Variables|DisplayProperties|GetAspectRatio) :NewEnumerator0 (Utilities|Struct|MakeIntPoint 36 36) :NewEnumerator1 (Utilities|Struct|MakeIntPoint 64 36) :NewEnumerator2 (Utilities|Struct|MakeIntPoint 84 36))))
  (bind _returnvalue (Rendering|CreateRenderTarget2D (.X (Utilities|Struct|BreakIntPoint _output_get)) (.Y (Utilities|Struct|BreakIntPoint _output_get)) "RTF_RGBA8" "(R=0.000000,G=0.000000,B=1.000000,A=1.000000)"))
  (bind _output_get_2 (Variables|Optimization|FoveatedCompression|SetFoveatedCompressionMaskRenderTarget _returnvalue))
  (Variables|/Script/Engine.Texture|SetLODGroup _output_get_2 "TEXTUREGROUP_Pixels2D")
  (Rendering|Material|SetTextureParameterValue (Variables|DisplayProperties|GetDMI_DisplayPlane_Inner) "Mask" "/Game/BP/ScreenBroadcasting/FoveatedCompression/RT_FoveatedMask.RT_FoveatedMask"))

(fn SortFoveatedCompressionMaskChannels
  (params (MaskPixels :type Array%20of%20Color%20Structures) (DisplayPixels :type Array%20of%20Color%20Structures) (PixelScaleFactor :type Integer) (TargetChannel :type E_ColorChannel%20Enum :default "NewEnumerator0"))
  (bind _returnvalue (Utilities|Array|Length MaskPixels))
  (Utilities|Array|Clear (LocalVariables|GetTempMaskedPixelArray))
  (Development|PrintString (Utilities|String|ToString(Integer) _returnvalue))
  (for _index (range 0 (- _returnvalue 1))
    (LocalVariables|SetCurrentPixelIndex _index)
    (switch Utilities|FlowControl|Switch|SwitchonE_ColorChannel TargetChannel))
  (return (LocalVariables|GetTempMaskedPixelArray)))

(fn SortFoveatedCompressionMaskChannelsData
  (params (Pixels :type Pixel%20Data%20Structure))
  (for _index (range 0 (- (* (Class|PixelReaderLibrary|GetWidth Pixels) (Class|PixelReaderLibrary|GetHeight Pixels)) 1))
    (LocalVariables|SetCurrentPixelIndex _index)
    (Utilities|FlowControl|Sequence
      (:then_0
        (if (== (.b (.Pixel (Class|PixelReaderLibrary|GetPixel Pixels (Utilities|Struct|MakeIntPoint (LocalVariables|GetCurrentX) (LocalVariables|GetCurrentY))))) 255)
          (Utilities|Array|Add (LocalVariables|GetPixelArray_B) (Math|Color|MakeColor 255 0 0 0))
          (Utilities|Array|Add (LocalVariables|GetPixelArray_G) (Math|Color|MakeColor 0 0 0 0))
          (Utilities|Array|Add (LocalVariables|GetPixelArray_R) (Math|Color|MakeColor 0 0 0 0))
          (elif (== (.g (.Pixel (Class|PixelReaderLibrary|GetPixel Pixels (Utilities|Struct|MakeIntPoint (LocalVariables|GetCurrentX) (LocalVariables|GetCurrentY))))) 255)
            (Utilities|Array|Add (LocalVariables|GetPixelArray_G) (Math|Color|MakeColor 0 255 0 0))
            (Utilities|Array|Add (LocalVariables|GetPixelArray_B) (Math|Color|MakeColor 0 0 0 0))
            (Utilities|Array|Add (LocalVariables|GetPixelArray_R) (Math|Color|MakeColor 0 0 0 0))
            (elif (== (.r (.Pixel (Class|PixelReaderLibrary|GetPixel Pixels (Utilities|Struct|MakeIntPoint (LocalVariables|GetCurrentX) (LocalVariables|GetCurrentY))))) 255)
              (Utilities|Array|Add (LocalVariables|GetPixelArray_R) (Math|Color|MakeColor 0 0 255 0))
              (Utilities|Array|Add (LocalVariables|GetPixelArray_B) (Math|Color|MakeColor 0 0 0 0))
              (Utilities|Array|Add (LocalVariables|GetPixelArray_G) (Math|Color|MakeColor 0 0 0 0))))))
      (:then_1
        ;[0 0 0] Increment pixel coordinates
        (if (== (- (Class|PixelReaderLibrary|GetWidth Pixels) 1) (LocalVariables|GetCurrentX))
          (LocalVariables|SetCurrentX 0)
          (Math|Integer|IncrementInt (LocalVariables|GetCurrentY))
          (else
            (Math|Integer|IncrementInt (LocalVariables|GetCurrentX)))))))
  (return (LocalVariables|GetPixelArray_B) (LocalVariables|GetPixelArray_G) (LocalVariables|GetPixelArray_R)))

(fn SwitchMaskedDisplayChannel
  (params (ColorChannel :type E_ColorChannel%20Enum :default "NewEnumerator0"))
  (Rendering|Material|SetScalarParameterValue (Variables|DisplayProperties|GetDMI_DisplayPlane_Inner) "RedMask" (Utilities|Select :Index ColorChannel :NewEnumerator0 1.0 :NewEnumerator1 0.0 :NewEnumerator2 0.0) :!class /Script/Engine.MaterialInstanceDynamic)
  (Rendering|Material|SetScalarParameterValue (Variables|DisplayProperties|GetDMI_DisplayPlane_Inner) "GreenMask" (Utilities|Select :Index ColorChannel :NewEnumerator0 0.0 :NewEnumerator1 1.0 :NewEnumerator2 0.0) :!class /Script/Engine.MaterialInstanceDynamic)
  (Rendering|Material|SetScalarParameterValue (Variables|DisplayProperties|GetDMI_DisplayPlane_Inner) "BlueMask" (Utilities|Select :Index ColorChannel :NewEnumerator0 0.0 :NewEnumerator1 0.0 :NewEnumerator2 1.0) :!class /Script/Engine.MaterialInstanceDynamic))